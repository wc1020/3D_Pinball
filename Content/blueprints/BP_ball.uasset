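; BP_ball is a physics ball actor that propels itself along the world X axis and clings to the surface beneath it.
; Each tick it scales audio volume and pitch by velocity, clamping both.
; It applies a Speed impulse, then traces downward and pushes the ball against the hit normal by Stickness.
; Both impulses are scaled by delta time and applied as velocity changes.
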(event EventBeginPlay)

(event EventTick
  (params (DeltaSeconds :type Float%20%28single-precision%29))
  (bind _returnvalue (Transformation|GetActorLocation))
  (bind _returnvalue_2 (Transformation|GetVelocity))
  (bind _audio (Variables|Default|GetAudio))
  (bind _returnvalue_3 (Math|Vector|VectorLength _returnvalue_2))
  (bind _returnvalue_4 (/ _returnvalue_3 2e+03))
  (Utilities|FlowControl|Sequence
    (:then_0
      (Audio|Components|Audio|SetVolumeMultiplier _audio (Math|Float|Clamp(Float) _returnvalue_4) :!class /Script/Engine.AudioComponent)
      (Audio|Components|Audio|SetPitchMultiplier _audio (Math|Float|Clamp(Float) _returnvalue_4 0.9 1.1)))
    (:then_1
      (Physics|AddImpulse (Variables|Default|Getball) (Math|Vector|MakeVector (* DeltaSeconds (Variables|Default|Getspeed)) 0.0 0.0) "None" true)
      (bind _outhit (Collision|LineTraceByChannel _returnvalue (- _returnvalue "0, 0,500.000000") "TraceTypeQuery1" false 0 "None"))
      (Physics|AddImpulse (Variables|Default|Getball) (* (* (* (.impactnormal _outhit) -1) (Variables|Default|Getstickness)) DeltaSeconds) "None" true))))

(fn ConstructionScript)